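; BP_SaveSettings is a data holder for video settings, storing console commands and option indices for graphics quality, frame rate, resolution and related options.
; SetSettings writes all values at once, while ReturnCommans and RetunInt read back the commands and indices separately.
; RetunInt outputs AAIndex for both PPIndex and AAIndex, so the stored post-process index is never returned.
; The file itself neither executes commands nor writes to disk.
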(fn SetSettings
  (params (FPSCommands :type String) (GraphicalCommands :type String) (PPComands :type String) (AACommands :type String) (ShadowsCommands :type String) (ResolutionCommands :type String) (TextureCommands :type String) (GraphicIndex :type Integer) (PPIndex :type Integer) (AAIndex :type Integer) (ShadowsIndex :type Integer) (TexturesIndex :type Integer) (RefrshRateIndex :type Integer) (Resolutionindex :type Integer))
  (Variables|Commands|SetFPSCommands FPSCommands)
  (Variables|Commands|SetGraphicalCommands GraphicalCommands)
  (Variables|Commands|SetPPComands PPComands)
  (Variables|Commands|SetAACommands AACommands)
  (Variables|Commands|SetShadowsCommands ShadowsCommands)
  (Variables|Commands|SetResolutionCommands ResolutionCommands)
  (Variables|Commands|SetTextureCommands TextureCommands)
  (Variables|Int|SetGraphicIndex GraphicIndex)
  (Variables|Int|SetPPIndex PPIndex)
  (Variables|Int|SetAAIndex AAIndex)
  (Variables|Int|SetShadowsIndex ShadowsIndex)
  (Variables|Int|SetTexturesIndex TexturesIndex)
  (Variables|Int|SetRefrshRateIndex RefrshRateIndex)
  (Variables|Int|SetResolutionIndex Resolutionindex))

(fn ReturnCommans
  (return (Variables|Commands|GetFPSCommands) (Variables|Commands|GetGraphicalCommands) (Variables|Commands|GetPPComands) (Variables|Commands|GetAACommands) (Variables|Commands|GetShadowsCommands) (Variables|Commands|GetTextureCommands) (Variables|Commands|GetResolutionCommands)))

(fn RetunInt
  (return (Variables|Int|GetGraphicIndex) (Variables|Int|GetAAIndex) (Variables|Int|GetAAIndex) (Variables|Int|GetShadowsIndex) (Variables|Int|GetTexturesIndex) (Variables|Int|GetRefrshRateIndex) (Variables|Int|GetResolutionIndex)))