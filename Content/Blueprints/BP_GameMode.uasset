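; Game mode for a runner game that handles level progression, game over and completion screens.
; BeginPlay caches the runner and finds the current level in the Levels array to set NextLevel or "END".
; EndGame slows time and shows game over; LevelComplete shows its widget, then a timer opens the next level or game-complete screen.
; BeginPlay's tile-spawn loop calls an empty function; a separate Spawnnexttile event spawns tiles.
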(event Custom|BreakLoop
  (bind _levels (Variables|Default|GetLevels))
  (bind _returnvalue (Utilities|Array|Length _levels))
  (bind _returnvalue_2 (- _returnvalue 1))
  ;[1 0.1971 0.8063] Level progression
  (Utilities|Array|ForEachLoopwithBreak _levels) ; enters at Break
)

(event Custom|Spawnnexttile
  (bind _returnvalue (Game|SpawnActorfromClass "/Game/Blueprints/Emviroment/BP_MasterTile.BP_MasterTile_C" (Math|Transform|MakeTransform (Variables|Default|GetSpawn%20Transform%20Location) "0, 0, 0" "1,1,1") "AlwaysSpawn" 0 0))
  (Variables|Default|SetSpawnTrasnform (Math|Transform|MakeTransform (Transformation|GetWorldLocation (Variables|/Game/Blueprints/Emviroment/BP_MasterTile.BP_MasterTile_C|GetSpawnPoint _returnvalue)) "0, 0, 0" "1,1,1")))

(event EventBeginPlay
  (bind _returnvalue (Game|GetPlayerController 0))
  (bind _levels (Variables|Default|GetLevels))
  (bind _returnvalue_2 (Utilities|Array|Length _levels))
  (bind _returnvalue_3 (- _returnvalue_2 1))
  ;[1 0.1971 0.8063] Level progression
  (for _index (range 0 9)
    (CallFunction|FSpawnTile))
  (bind _asbp_runner (Utilities|Casting|CastToBP_Runner (Game|GetPlayerCharacter 0)))
  (Variables|Default|SetAs%20BP%20Runner _asbp_runner)
  (Variables|/Script/Engine.PlayerController|SetbShowMouseCursor _returnvalue false)
  (Input|SetInputModeGameOnly _returnvalue)
  (bind _returnvalue_4 (Game|GetCurrentLevelName true))
  (bind (_array_element _array_index) (Utilities|Array|ForEachLoopwithBreak _levels)
    (:LoopBody
      (Variables|Default|SetcurrentIndex _array_index)
      (if (and (Utilities|Enum|Equal(Enum) _array_element _returnvalue_4) (< (Variables|Default|GetcurrentIndex) _returnvalue_3))
        (Variables|Default|SetnextLevel (Utilities|Array|Get(acopy) (Variables|Default|GetLevels) (+ (Variables|Default|GetcurrentIndex) 1)))
        (CallFunction|BreakLoop)
        (elif (== (Variables|Default|GetcurrentIndex) _returnvalue_3)
          (Variables|Default|SetnextLevel "END")
          (CallFunction|BreakLoop))))))

(fn ConstructionScript)

(fn EndGame
  (bind _returnvalue (Game|GetPlayerController 0))
  (Utilities|Time|SetGlobalTimeDilation 0.25)
  (bind _returnvalue_2 (UserInterface|CreateWidget "/Game/Blueprints/UserInterface/WBP_GameOver.WBP_GameOver_C"))
  (UserInterface|Viewport|AddtoViewport _returnvalue_2 0)
  (Variables|/Script/Engine.PlayerController|SetbShowMouseCursor _returnvalue true)
  (Input|SetInputModeUIOnly _returnvalue _returnvalue_2 "DoNotLock"))

(fn LevelComplete
  (bind _returnvalue (UserInterface|CreateWidget "/Game/Blueprints/UserInterface/WBP_LevelComplete.WBP_LevelComplete_C"))
  (bind _output_get (Variables|Default|SetWBP_LevelComplete _returnvalue))
  (UserInterface|Viewport|AddtoViewport _output_get 0)
  (Utilities|Time|SetTimerbyFunctionName 0 "LoadNextLevel" 2.0))

(fn LoadNextLevel
  (bind _returnvalue (Game|GetPlayerController 0))
  (bind _wbp_levelcomplete (Variables|Default|GetWBP_LevelComplete))
  (if (Utilities|Enum|Equal(Enum) (Variables|Default|GetnextLevel) "END")
    (Utilities|IsValid _wbp_levelcomplete
      (:Is%20Valid
        (Widget|RemovefromParent _wbp_levelcomplete))
      (:Is%20Not%20Valid
        _))
    (bind _returnvalue_2 (UserInterface|CreateWidget "/Game/Blueprints/UserInterface/WBP_GameComplete.WBP_GameComplete_C"))
    (UserInterface|Viewport|AddtoViewport _returnvalue_2 0)
    (Variables|/Script/Engine.PlayerController|SetbShowMouseCursor _returnvalue true)
    (Input|SetInputModeUIOnly _returnvalue _returnvalue_2 "DoNotLock")
    (else
      (Game|OpenLevel(byName) (Utilities|String|StringToName (Variables|Default|GetnextLevel))))))

(fn FSpawnTile)