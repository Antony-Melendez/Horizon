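; Game mode for an endless runner that builds the tile track and handles game over.
; BeginPlay lays ten tiles by calling AddFloorTile, which chains each BP_MasterTile at the previous tile's spawn point transform.
; The random tile pick is currently limited to the first TilesToSpawn entry.
; EndGame slows global time, shows WBP_GameOver and switches to mouse-driven UI-only input.
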(event EventBeginPlay
  (for _index (range 0 9)
    (CallFunction|AddFloorTile)))

(fn ConstructionScript)

(fn AddFloorTile
  (bind _returnvalue (Game|SpawnActorfromClass (Utilities|Array|Get(acopy) (Variables|Default|GetTilesToSpawn) (Math|Random|RandomIntegerinRange 0 0)) (Variables|Default|GetNextSpawnTransform) "Undefined" 0 0))
  (bind _asbp_master_tile (Utilities|Casting|CastToBP_MasterTile _returnvalue))
  (bind _spawntransform (Default|GetSpawnPointTransform _asbp_master_tile))
  (Variables|Default|SetNextSpawnTransform _spawntransform))

(fn EndGame
  (bind _returnvalue (Game|GetPlayerController 0))
  (Utilities|Time|SetGlobalTimeDilation 0.25)
  (bind _returnvalue_2 (UserInterface|CreateWidget "/Game/Blueprints/UserInterface/WBP_GameOver.WBP_GameOver_C"))
  (UserInterface|Viewport|AddtoViewport _returnvalue_2 0)
  (Variables|/Script/Engine.PlayerController|SetbShowMouseCursor _returnvalue true)
  (Input|SetInputModeUIOnly _returnvalue _returnvalue_2 "DoNotLock"))