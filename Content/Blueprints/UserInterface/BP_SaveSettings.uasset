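; BP_SaveSettings is a data container for the player's graphics settings, covering quality, post-process, anti-aliasing, shadows, textures, FPS cap, resolution and screen mode.
; SetSettings stores a command and a selection index for each option.
; ReturnCommans hands back the commands, and RetunInt hands back the indices.
; RetunInt outputs AAIndex in the PPIndex slot, so the stored post-process index is never returned.
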(fn SetSettings
  (params (MaxFPSCommands :type String) (GraphicalCommands :type String) (PPComands :type String) (AACommands :type String) (ShadowsCommands :type String) (ResolutionCommands :type String) (TextureCommands :type String) (ScreenModeCommand :type String) (GraphicIndex :type Integer) (PPIndex :type Integer) (AAIndex :type Integer) (ShadowsIndex :type Integer) (TexturesIndex :type Integer) (MaxFPSIndex :type Integer) (Resolutionindex :type Integer) (ScreenModeIndex :type Integer))
  (Variables|Commands|SetFPSCommands MaxFPSCommands)
  (Variables|Commands|SetGraphicalCommands GraphicalCommands)
  (Variables|Commands|SetPPComands PPComands)
  (Variables|Commands|SetAACommands AACommands)
  (Variables|Commands|SetShadowsCommands ShadowsCommands)
  (Variables|Commands|SetResolutionCommands ResolutionCommands)
  (Variables|Commands|SetTextureCommands TextureCommands)
  (Variables|Commands|SetScreenModeCommands ScreenModeCommand)
  (Variables|Int|SetGraphicIndex GraphicIndex)
  (Variables|Int|SetPPIndex PPIndex)
  (Variables|Int|SetAAIndex AAIndex)
  (Variables|Int|SetShadowsIndex ShadowsIndex)
  (Variables|Int|SetTexturesIndex TexturesIndex)
  (Variables|Int|SetMaxFPSIndex MaxFPSIndex)
  (Variables|Int|SetResolutionIndex Resolutionindex)
  (Variables|Int|SetScreenModeIndex ScreenModeIndex))

(fn ReturnCommans
  (return (Variables|Commands|GetFPSCommands) (Variables|Commands|GetGraphicalCommands) (Variables|Commands|GetPPComands) (Variables|Commands|GetAACommands) (Variables|Commands|GetShadowsCommands) (Variables|Commands|GetTextureCommands) (Variables|Commands|GetResolutionCommands) (Variables|Commands|GetScreenModeCommands)))

(fn RetunInt
  (return (Variables|Int|GetGraphicIndex) (Variables|Int|GetAAIndex) (Variables|Int|GetAAIndex) (Variables|Int|GetShadowsIndex) (Variables|Int|GetTexturesIndex) (Variables|Int|GetMaxFPSIndex) (Variables|Int|GetResolutionIndex) (Variables|Int|GetScreenModeIndex)))